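; Trigger component for CARLA traffic lights that links vehicles in a stop box to the owning BP_TrafficLightNew.
; BindOverlap hooks the BoxCollider's overlap events, which add or remove wheeled vehicles in StoppedCars and notify or un-notify the light.
; New entries register only while the separate StoppedCar reference is invalid.
; When the light state changes, every vehicle in StoppedCars is notified again.
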(event `self.ReceiveBeginPlay`
  (bind _asbp_traffic_light_new (cast `/Game/Carla/Static/TrafficLight/Streetlights_01/BP_TrafficLightNew` (`self.GetOwner`)))
  (set `self.TrafficLight` _asbp_traffic_light_new))

(event `BindOverlap`
  (bind _stoppedcar (`self.StoppedCar`))
  (add `PrimitiveComponent.OnComponentBeginOverlap` (`self.BoxCollider`) (delegate `OnComponentBeginOverlap`))
  (add `PrimitiveComponent.OnComponentEndOverlap` (`self.BoxCollider`) (delegate `OnComponentEndOverlap`))
  (if (== (stale `OnComponentEndOverlap` OtherActor) _stoppedcar)
    (`TrafficLightBase.UnNotifyWheeledVehicle` (`self.TrafficLight`) _stoppedcar)
    (`KismetArrayLibrary.Array_RemoveItem` (`self.StoppedCars`) _stoppedcar)))

(event `OnComponentEndOverlap`
  (params (OverlappedComponent :type "PrimitiveComponent Object Reference") (OtherActor :type "Actor Object Reference") (OtherComp :type "PrimitiveComponent Object Reference") (OtherBodyIndex :type Integer))
  (`/Engine/EditorBlueprintResources/StandardMacros.IsValid` OtherActor
    (:`Is Valid`
      (bind _ascarla_wheeled_vehicle (cast `CarlaWheeledVehicle` OtherActor))
      (`TrafficLightBase.UnNotifyWheeledVehicle` (`self.TrafficLight`) _ascarla_wheeled_vehicle)
      (`KismetArrayLibrary.Array_RemoveItem` (`self.StoppedCars`) _ascarla_wheeled_vehicle))))

(event `OnComponentBeginOverlap`
  (params (OverlappedComponent :type "PrimitiveComponent Object Reference") (OtherActor :type "Actor Object Reference") (OtherComp :type "PrimitiveComponent Object Reference") (OtherBodyIndex :type Integer) (bFromSweep :type Boolean) (SweepResult :type "HitResult Structure (by ref)"))
  (`/Engine/EditorBlueprintResources/StandardMacros.IsValid` (`self.TrafficLight`)
    (:`Is Valid`
      (`/Engine/EditorBlueprintResources/StandardMacros.IsValid` (`self.StoppedCar`)
        (:`Is Not Valid`
          (bind _ascarla_wheeled_vehicle (cast `CarlaWheeledVehicle` OtherActor))
          (`KismetArrayLibrary.Array_Add` (`self.StoppedCars`) _ascarla_wheeled_vehicle)
          (`TrafficLightBase.NotifyWheeledVehicle` (`self.TrafficLight`) _ascarla_wheeled_vehicle))))))

(event `LightTrafficStateChanged`
  (params (LightState :type "ETrafficLightState Enum" :default "Red"))
  (for _array_element (`self.StoppedCars`)
    (`TrafficLightBase.NotifyWheeledVehicle` (`self.TrafficLight`) _array_element)))