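; Terraced house building actor for the Carla map, with toggleable lights and randomly placed props.
; The construction script calls PlaceItems to spawn air conditioner meshes from a positions array, with spawn and random-position options.
; On the BP_Lights ChangeLight event, it passes four point lights to BPLights for updating and sets the emissive on the ground floor mesh.
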(event `self.BP_Lights.ChangeLight`
  (bind _bp_lights (`self.BP_Lights`))
  (`/Game/Carla/Blueprints/Lights/BP_Lights.SetLight` _bp_lights (`self.PointLight`))
  (`/Game/Carla/Blueprints/Lights/BP_Lights.SetLight` _bp_lights (`self.PointLight1`))
  (`/Game/Carla/Blueprints/Lights/BP_Lights.SetLight` _bp_lights (`self.PointLight4`))
  (`/Game/Carla/Blueprints/Lights/BP_Lights.SetLight` _bp_lights (`self.PointLight5`))
  (`/Game/Carla/Blueprints/Lights/BP_Lights.SetEmissive` _bp_lights (`self.GroundFloor`)))

(fn `UserConstructionScript`
  (`parent.UserConstructionScript`)
  (`self.PlaceItems` (`self.SpawnAny`) (`self.AirConditioners`) (`self.PositionsArray`) (`self.RandomPositions`)))