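; Double street light actor for Carla, with two spot lights, a point light and an emissive lamp mesh.
; On the ChangeLight event it passes all three lights and the mesh to BPLights, which sets the lights and the emissive.
; It then overrides the point light's intensity to a third of the intensity BPLights reports.
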(event `self.BP_Lights.ChangeLight`
  (bind _pointlight (`self.PointLight`))
  (bind _bp_lights (`self.BP_Lights`))
  (`/Game/Carla/Blueprints/Lights/BP_Lights.SetLight` _bp_lights (`self.SpotLight`))
  (`/Game/Carla/Blueprints/Lights/BP_Lights.SetLight` _bp_lights (`self.SpotLight1`))
  (`/Game/Carla/Blueprints/Lights/BP_Lights.SetLight` _bp_lights _pointlight)
  (`/Game/Carla/Blueprints/Lights/BP_Lights.SetEmissive` _bp_lights (`self.StreetLight_Mesh`))
  (`LightComponent.SetIntensity` _pointlight (/ (`CarlaLight.GetLightIntensity` _bp_lights) 3.0)))

(fn `UserConstructionScript`)