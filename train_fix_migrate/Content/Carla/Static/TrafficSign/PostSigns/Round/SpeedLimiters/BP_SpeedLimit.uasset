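; Speed limit traffic sign that applies its SpeedLimit to vehicles entering its trigger Box.
; On overlap, SendSpeedLimit casts the actor to BaseVehiclePawn and calls SetSpeedLimit on its WheeledVehicleAIController, ignoring anything else.
; Helper functions return the Box or reposition it in world space, with YRot feeding yaw and ZRot feeding pitch.
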(event `self.Box.OnComponentBeginOverlap`
  (params (OverlappedComponent :type "PrimitiveComponent Object Reference") (OtherActor :type "Actor Object Reference") (OtherComp :type "PrimitiveComponent Object Reference") (OtherBodyIndex :type Integer) (bFromSweep :type Boolean) (SweepResult :type "HitResult Structure (by ref)"))
  (`self.SendSpeedLimit` OtherActor (`self.SpeedLimit`)))

(fn `GetTriggerVolume`
  (returns (ReturnValue :type "BoxComponent Object Reference"))
  (return (`self.Box`)))

(fn `SendSpeedLimit`
  (params (Object :type "Object Object Reference") (SpeedLimit :type "Float (double-precision)"))
  (bind _asbase_vehicle_pawn (cast `/Game/Carla/Blueprints/Vehicles/BaseVehiclePawn` Object))
  (bind _aswheeled_vehicle_aicontroller (cast `WheeledVehicleAIController` (`Pawn.GetController` _asbase_vehicle_pawn)))
  (`WheeledVehicleAIController.SetSpeedLimit` _aswheeled_vehicle_aicontroller SpeedLimit))

(fn `SetBoxLocationAndRotation`
  (params (xPos :type "Float (double-precision)") (yPos :type "Float (double-precision)") (zPos :type "Float (double-precision)") (xRot :type "Float (double-precision)") (yRot :type "Float (double-precision)") (zRot :type "Float (double-precision)"))
  (`SceneComponent.K2_SetWorldLocationAndRotation` (`self.Box`) (`KismetMathLibrary.MakeVector` xPos yPos zPos) (`KismetMathLibrary.MakeRotator` xRot zRot yRot) false false))

(fn `UserConstructionScript`)