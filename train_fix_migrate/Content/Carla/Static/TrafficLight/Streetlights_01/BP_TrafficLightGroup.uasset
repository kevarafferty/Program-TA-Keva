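; BP_TrafficLightGroup turns a list of placed CARLA traffic lights into a runtime TrafficLightGroup.
; On BeginPlay it spawns the group, gives each light a pole index and its own controller, and resets the group.
; It then registers each light component with the game mode's TrafficLightManager.
; A separate UpdateTrafficLights function, not called in this Blueprint, cycles round-robin by unfreezing the next light when the selected one is frozen on red.
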(event `self.ReceiveBeginPlay`
  (bind _returnvalue (`|SpawnActorFromClass` "/Script/Carla.TrafficLightGroup" (`self.GetTransform`) "Undefined" "OverrideRootScale" null null))
  (for (_array_element _array_index) (`self.TrafficLights`)
    (`TrafficLightBase.SetPoleIndex` _array_element _array_index)
    (bind _returnvalue_2 (`|GenericCreateObject` "/Script/Carla.TrafficLightController" _returnvalue))
    (`TrafficLightController.AddTrafficLight` _returnvalue_2 (`TrafficLightBase.GetTrafficLightComponent` _array_element))
    (`TrafficLightGroup.AddController` _returnvalue _returnvalue_2))
  (`TrafficLightGroup.ResetGroup` _returnvalue)
  (bind _returnvalue_3 (`CarlaGameModeBase.GetTrafficLightManager` (`CarlaStatics.GetGameMode`)))
  (for _array_element_2 (`self.TrafficLights`)
    (`TrafficLightManager.RegisterLightComponentGenerated` _returnvalue_3 (`TrafficLightBase.GetTrafficLightComponent` _array_element_2))))

(fn `UpdateTrafficLights`
  (params (deltaTime :type "Float (double-precision)"))
  (bind _trafficlights (`self.TrafficLights`))
  (bind _output (`|GetArrayItem` _trafficlights (`self.SelectedTrafficLight`)))
  ;[1 1 1] WTF!!!!!!!!!
  (if (> (`KismetArrayLibrary.Array_Length` _trafficlights) 0)
    (if (and (`TrafficLightBase.GetTimeIsFrozen` _output) (`|EnumEquality` "Red" (`TrafficLightBase.GetTrafficLightState` _output)))
      (bind _result (`/Engine/EditorBlueprintResources/StandardMacros.IncrementInt` (`self.SelectedTrafficLight`))
        (:`  `
          (if (== _result (`KismetArrayLibrary.Array_Length` (`self.TrafficLights`)))
            (set `self.SelectedTrafficLight` 0))
          (`TrafficLightBase.SetTimeIsFrozen` (`|GetArrayItem` (`self.TrafficLights`) (`self.SelectedTrafficLight`)) false))))))

(fn `UserConstructionScript`)