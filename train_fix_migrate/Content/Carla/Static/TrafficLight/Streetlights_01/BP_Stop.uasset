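; BP_Stop is a CARLA stop or yield sign that holds AI vehicles at a junction by setting their controllers' traffic light state.
; CheckBox tracks vehicles in the area; StopBox holds arrivals red while it is occupied.
; Once clear, yield releases vehicles immediately, while stop queues them on a StopTime countdown in Tick before turning green.
; The construction script sets the billboard and sign state, reporting UNKNOWN when hidden from the Python API.
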(event `self.CheckBox.OnComponentBeginOverlap`
  (params (OverlappedComponent :type "PrimitiveComponent Object Reference") (OtherActor :type "Actor Object Reference") (OtherComp :type "PrimitiveComponent Object Reference") (OtherBodyIndex :type Integer) (bFromSweep :type Boolean) (SweepResult :type "HitResult Structure (by ref)"))
  (`|ExecutionSequence`
    (:`then_1`
      (`/Engine/EditorBlueprintResources/StandardMacros.IsValid` OtherActor
        (:`Is Valid`
          (cast `CarlaWheeledVehicle` OtherActor)
          (`KismetArrayLibrary.Array_Add` (`self.Vehicles in area array`) OtherActor))))))

(event `self.CheckBox.OnComponentEndOverlap`
  (params (OverlappedComponent :type "PrimitiveComponent Object Reference") (OtherActor :type "Actor Object Reference") (OtherComp :type "PrimitiveComponent Object Reference") (OtherBodyIndex :type Integer))
  (bind _vehicles_in_area_array (`self.Vehicles in area array`))
  (`/Engine/EditorBlueprintResources/StandardMacros.IsValid` OtherActor
    (:`Is Valid`
      (cast `CarlaWheeledVehicle` OtherActor)
      (`KismetArrayLibrary.Array_RemoveItem` _vehicles_in_area_array OtherActor)
      (if (<= (`KismetArrayLibrary.Array_Length` _vehicles_in_area_array) 1)
        (for _array_element (`self.StoredStoppedVehicles`)
          (bind _returnvalue (`Pawn.GetController` _array_element))
          (`/Engine/EditorBlueprintResources/StandardMacros.IsValid` _returnvalue
            (:`Is Valid`
              (bind _aswheeled_vehicle_aicontroller (cast `WheeledVehicleAIController` _returnvalue))
              (if (> (`KismetArrayLibrary.Array_Length` _vehicles_in_area_array) 0)
                (`WheeledVehicleAIController.SetTrafficLightState` _aswheeled_vehicle_aicontroller "Red")
                (elif (`self.Stop/Yield`)
                  (`WheeledVehicleAIController.SetTrafficLightState` _aswheeled_vehicle_aicontroller "Red")
                  (`KismetArrayLibrary.Array_Add` (`self.Vehicle_Time`) (make `/Game/Carla/Blueprints/Tools/Vehicle_Time_Pair` _aswheeled_vehicle_aicontroller (`self.StopTime`)))
                  (else
                    (`/Engine/EditorBlueprintResources/StandardMacros.IsValid` _aswheeled_vehicle_aicontroller
                      (:`Is Valid`
                        (`WheeledVehicleAIController.SetTrafficLightState` _aswheeled_vehicle_aicontroller "Green")))))))))))))

(event `self.ReceiveTick`
  (params (DeltaSeconds :type "Float (single-precision)"))
  (bind _vehicle_time (`self.Vehicle_Time`))
  (for (_array_element _array_index) _vehicle_time
    (`KismetArrayLibrary.Array_Set` (`self.Vehicle_Time`) _array_index (make `/Game/Carla/Blueprints/Tools/Vehicle_Time_Pair` (break `/Game/Carla/Blueprints/Tools/Vehicle_Time_Pair` _array_element) (- (`.Time_5_83E7BA131957409DB275B584D55ED0EF` (break `/Game/Carla/Blueprints/Tools/Vehicle_Time_Pair` _array_element)) DeltaSeconds))))
  (bind (_arrayindex _arrayelement) (`/Engine/EditorBlueprintResources/StandardMacros.ReverseForEachLoop` _vehicle_time)
    (:`LoopBody`
      (bind (_vehicle _time) (break `/Game/Carla/Blueprints/Tools/Vehicle_Time_Pair` _arrayelement))
      (if (< _time 0.0)
        (`/Engine/EditorBlueprintResources/StandardMacros.IsValid` _vehicle
          (:`Is Valid`
            (`WheeledVehicleAIController.SetTrafficLightState` _vehicle "Green")
            (`KismetArrayLibrary.Array_Remove` (`self.Vehicle_Time`) _arrayindex)))))))

(event `self.StopBox.OnComponentBeginOverlap`
  (params (OverlappedComponent :type "PrimitiveComponent Object Reference") (OtherActor :type "Actor Object Reference") (OtherComp :type "PrimitiveComponent Object Reference") (OtherBodyIndex :type Integer) (bFromSweep :type Boolean) (SweepResult :type "HitResult Structure (by ref)"))
  (`|ExecutionSequence`
    (:`then_1`
      (`/Engine/EditorBlueprintResources/StandardMacros.IsValid` OtherActor
        (:`Is Valid`
          (bind _ascarla_wheeled_vehicle (cast `CarlaWheeledVehicle` OtherActor))
          (`KismetArrayLibrary.Array_Add` (`self.StoredStoppedVehicles`) _ascarla_wheeled_vehicle)
          (bind _returnvalue (`Pawn.GetController` _ascarla_wheeled_vehicle))
          (`/Engine/EditorBlueprintResources/StandardMacros.IsValid` _returnvalue
            (:`Is Valid`
              (bind _aswheeled_vehicle_aicontroller (cast `WheeledVehicleAIController` _returnvalue))
              (if (> (`KismetArrayLibrary.Array_Length` (`self.Vehicles in area array`)) 0)
                (`WheeledVehicleAIController.SetTrafficLightState` _aswheeled_vehicle_aicontroller "Red")
                (elif (`self.Stop/Yield`)
                  (`WheeledVehicleAIController.SetTrafficLightState` _aswheeled_vehicle_aicontroller "Red")
                  (`KismetArrayLibrary.Array_Add` (`self.Vehicle_Time`) (make `/Game/Carla/Blueprints/Tools/Vehicle_Time_Pair` _aswheeled_vehicle_aicontroller (`self.StopTime`)))
                  (else
                    (`/Engine/EditorBlueprintResources/StandardMacros.IsValid` _aswheeled_vehicle_aicontroller
                      (:`Is Valid`
                        (`WheeledVehicleAIController.SetTrafficLightState` _aswheeled_vehicle_aicontroller "Green")))))))))))))

(event `self.StopBox.OnComponentEndOverlap`
  (params (OverlappedComponent :type "PrimitiveComponent Object Reference") (OtherActor :type "Actor Object Reference") (OtherComp :type "PrimitiveComponent Object Reference") (OtherBodyIndex :type Integer))
  (`/Engine/EditorBlueprintResources/StandardMacros.IsValid` OtherActor
    (:`Is Valid`
      (bind _ascarla_wheeled_vehicle (cast `CarlaWheeledVehicle` OtherActor))
      (bind _returnvalue (`Pawn.GetController` _ascarla_wheeled_vehicle))
      (`/Engine/EditorBlueprintResources/StandardMacros.IsValid` _returnvalue
        (:`Is Valid`
          (bind _aswheeled_vehicle_aicontroller (cast `WheeledVehicleAIController` _returnvalue))
          (`WheeledVehicleAIController.SetTrafficLightState` _aswheeled_vehicle_aicontroller "Green")
          (`KismetArrayLibrary.Array_RemoveItem` (`self.StoredStoppedVehicles`) _ascarla_wheeled_vehicle))))))

(fn `GetTriggerVolume`
  (returns (ReturnValue :type "BoxComponent Object Reference"))
  (return (`self.StopBox`)))

(fn `UserConstructionScript`
  (bind _billboard (`self.Billboard`))
  (if (`self.Stop/Yield`)
    (`BillboardComponent.SetSprite` _billboard "/Game/Carla/Static/GenericMaterials/Icons/Stop.Stop")
    (`self.SetTrafficSignState` "StopSign")
    (else
      (`BillboardComponent.SetSprite` _billboard "/Game/Carla/Static/GenericMaterials/Icons/Yield.Yield")
      (`self.SetTrafficSignState` "YieldSign")))
  (if (`self.hidden in PythonAPI`)
    (`self.SetTrafficSignState` "UNKNOWN")))